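; Enemy Blueprint with a montage-driven melee attack whose blade overlap damages the player while attacking.
; Taking damage updates HP and its widget bar, plays a hit montage and shows damage text, with a brief lockout against repeat hits.
; If IsParry is set when damaged, a short global time-dilation hit stop precedes a parried montage and knockback launch.
; At zero HP it ragdolls, hides, spawns a Niagara death effect and destroys itself.
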(event OnComponentBeginOverlap(BladeCollision)
  (params (OverlappedComponent :type Primitive%20Component%20Object%20Reference) (OtherActor :type Actor%20Object%20Reference) (OtherComp :type Primitive%20Component%20Object%20Reference) (OtherBodyIndex :type Integer) (bFromSweep :type Boolean) (SweepResult :type Hit%20Result%20Structure%20%28by%20ref%29))
  ;[1 1 1] Damage
  (if (and (== OtherActor (Game|Player|GetPlayerPawn 0)) (Variables|Default|GetIsAttack))
    (Game|Damage|ApplyDamage OtherActor (Variables|Default|GetAttackDamage) 0 0)))

(event Custom|Attack
  ;[1 0 0 0.5] 攻撃
  (Animation|Montage|PlayMontage (Variables|Character|GetMesh) "/Game/UnrealQuest5/Characters/Mannequins/Animations/UQ5/AM_Enemy_Attack01.AM_Enemy_Attack01"
    (:then
      (Variables|Default|SetIsAttack true))
    (:OnCompleted
      (Variables|Default|SetIsAttack false :!label _label))
    (:OnBlendOut
      (goto _label))
    (:OnInterrupted
      (goto _label))))

(event Custom|Dead
  (bind _mesh (Variables|Character|GetMesh))
  (bind _mesh_2 (Variables|Character|GetMesh))
  ;[1 1 1] Dead
  (Variables|Default|SetIsAttack false)
  (Variables|Actor|SetbCanBeDamaged false)
  (Collision|SetCollisionProfileName _mesh "Ragdoll" true :!class /Script/Engine.PrimitiveComponent)
  (Class|SkeletalMeshComponent|SetAllBodiesSimulatePhysics _mesh true)
  (Utilities|FlowControl|Delay 1.5)
  (Rendering|SetVisibility _mesh_2 false false)
  (Niagara|SpawnSystemAttached "/Game/UnrealQuest5/Effects/NS_Dead.NS_Dead" _mesh_2 "None" "0, 0, 0" "0, 0, 0" "KeepRelativeOffset" false)
  (Utilities|FlowControl|Delay 4.0)
  (Actor|DestroyActor))

(event Custom|Parry
  ;[1 1 1] Parry
  (if (Variables|Default|GetIsParry)
    (Utilities|FlowControl|Delay 0.05)
    (Utilities|Time|SetGlobalTimeDilation 0.05)
    (Utilities|FlowControl|Delay 0.025)
    (Utilities|Time|SetGlobalTimeDilation 1.0)
    (Animation|Montage|PlayMontage (Variables|Character|GetMesh) "/Game/UnrealQuest5/Characters/Mannequins/Animations/UQ5/AM_GotParried.AM_GotParried"
      (:then
        (Character|LaunchCharacter (* (Transformation|GetActorForwardVector) -1000) true true)))))

(event Custom|DamagedText
  (params (Damage :type Float%20%28double-precision%29))
  ;[1 1 1] DamagedText
  (bind _returnvalue (UserInterface|CreateWidget "/Game/UnrealQuest5/Blueprints/WBP_Damage.WBP_Damage_C" 0 self Damage))
  (UserInterface|Viewport|AddtoViewport _returnvalue 0))

(event Game|Damage|EventAnyDamage
  (params (Damage :type Float%20%28single-precision%29) (DamageType :type Damage%20Type%20Object%20Reference) (InstigatedBy :type Controller%20Object%20Reference) (DamageCauser :type Actor%20Object%20Reference))
  ;[1 1 1] Damaged
  (CallFunction|Parry)
  (if (not (Variables|Default|GetIsDamage))
    (Variables|Default|SetIsDamage true)
    (Variables|Default|SetEnemyHP (- (Variables|Default|GetEnemyHP) Damage))
    (bind _aswbp_enemy_hp (Utilities|Casting|CastToWBP_EnemyHP (UserInterface|GetWidget (Variables|Default|GetWidget))))
    (Default|UpdateEnemyHPBar _aswbp_enemy_hp (Variables|Default|GetEnemyHP) (Variables|Default|GetEnemyMaxHP))
    (Utilities|FlowControl|Sequence
      (:then_0
        (Animation|Montage|PlayMontage (Variables|Character|GetMesh) "/Game/UnrealQuest5/Characters/Mannequins/Animations/UQ5/AM_Damaged.AM_Damaged"
          (:then
            (if (<= (Variables|Default|GetEnemyHP) 0.0)
              (CallFunction|Dead)))))
      (:then_1
        (CallFunction|DamagedText Damage))
      (:then_2
        (Utilities|FlowControl|Delay 0.4)
        (Variables|Default|SetIsDamage false)))))

(fn ConstructionScript)